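; BP_KeyPickup is a key pickup that grants the player a key identified by KeyIndex.
; Its PlayerPickup event passes that index to the player's AddKey.
; The construction script creates a dynamic instance of M_TestDoor on the mesh and sets its KeyColor parameter from GetKeyColor, so each key is tinted by its index.
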(event EventBeginPlay
  (|CallParentFunction) ; This node is disabled and will not be called.\nDrag off pins to build functionality.
)

(event Collision|EventActorBeginOverlap
  (params (OtherActor :type Actor%20Object%20Reference))
  (|CallParentFunction OtherActor) ; This node is disabled and will not be called.\nDrag off pins to build functionality.
)

(event EventTick
  (params (DeltaSeconds :type Float%20%28single-precision%29)))

(event EventPlayerPickup
  (params (Player :type BP%20First%20Person%20Character%20Object%20Reference))
  (Default|AddKey Player (Variables|Default|GetKeyIndex)))

(fn ConstructionScript
  (|CallParentFunction)
  (bind _returnvalue (Rendering|Material|CreateDynamicMaterialInstance (Variables|Character|GetMesh) 0 "/Game/BoomerShooter/Blueprints/Doors/M_TestDoor.M_TestDoor" "None" :!class /Script/Engine.PrimitiveComponent))
  (Rendering|Material|SetVectorParameterValue _returnvalue "KeyColor" (CallFunction|GetKeyColor (Variables|Default|GetKeyIndex)) :!class /Script/Engine.MaterialInstanceDynamic))