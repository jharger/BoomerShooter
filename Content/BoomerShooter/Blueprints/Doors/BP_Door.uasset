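; Keyed door for a boomer shooter that slides upward when the player interacts with it.
; The construction script tints a dynamic material with the color for its KeyIndex.
; CanInteract and the prompt check the player's key, with a plain open prompt for negative indices.
; Interact runs once, using the key, blacking out the key color, then raising the door on a timeline after a short delay.
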(event EventBeginPlay
  (Utilities|FlowControl|Sequence
    (:then_0
      (Variables|Default|SetStartLocation (Transformation|GetActorLocation)))))

(event EventInteract
  (params (Character :type BP%20First%20Person%20Character%20Object%20Reference))
  (Utilities|FlowControl|DoOnce false
    (:Completed
      (Default|UseKey Character (Variables|Door|GetKeyIndex))
      (Rendering|Material|SetVectorParameterValue :self (Variables|Default|GetMaterial) :ParameterName "KeyColor" :!class /Script/Engine.MaterialInstanceDynamic)
      (Utilities|FlowControl|Delay 0.2)
      (bind _progress (Timeline|DoorOpen PlayFromStart)
        (:Update
          (Transformation|SetActorLocation (+ (* (Math|Vector|VectorUp) _progress (Variables|Default|GetOpenHeight)) (Variables|Default|GetStartLocation)) false false))))))

(fn ConstructionScript
  (bind _returnvalue (Rendering|Material|CreateDynamicMaterialInstance (Variables|Default|GetCube) 0 "/Game/BoomerShooter/Blueprints/Doors/M_TestDoor.M_TestDoor" "None" :!class /Script/Engine.PrimitiveComponent))
  (bind _output_get (Variables|Default|SetMaterial _returnvalue))
  (Rendering|Material|SetVectorParameterValue _output_get "KeyColor" (CallFunction|GetKeyColor (Variables|Door|GetKeyIndex)) :!class /Script/Engine.MaterialInstanceDynamic))

(fn CanInteract
  (params (Player :type BP%20First%20Person%20Character%20Object%20Reference))
  (return (Default|HasKey Player (Variables|Door|GetKeyIndex))))

(fn GetInteractMessage
  (params (Player :type BP%20First%20Person%20Character%20Object%20Reference))
  (bind _keyindex (Variables|Door|GetKeyIndex))
  (bind _name (CallFunction|GetKeyName _keyindex))
  (if (< (Variables|Door|GetKeyIndex) 0)
    (return "Open Door")
    (else
      (return (Utilities|String|SelectText (Utilities|Text|FormatText "Open Door ({keyName} Key})" _name) (Utilities|Text|FormatText "Locked ({keyName} Key})" _name) (Default|HasKey Player _keyindex))))))